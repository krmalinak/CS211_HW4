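; Self-propelled rocket projectile that explodes on contact or after a fuse time.
; Tick adds velocity to the physics-driven static mesh along the actor's forward axis, unscaled by delta time.
; Overlaps and mesh hits share one path: spawn the explosion emitter, send ProjectileHitObjectMessage to the other actor, then destroy.
; Timeout from BeginPlay explodes without notifying anything; the separate Explode function is not called here.
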(event OnComponentHit(StaticMesh)
  (params (OtherActor :type Actor%20Object%20Reference) (OtherComp :type Primitive%20Component%20Object%20Reference) (NormalImpulse :type Vector :default "0, 0, 0") (Hit :type Hit%20Result%20Structure%20%28by%20ref%29))
  (Effects|SpawnEmitteratLocation "/Game/StarterContent/Particles/P_Explosion.P_Explosion" (Transformation|GetWorldLocation (Variables|Default|GetStaticMesh)))
  (Class|BPIExplodable|ProjectileHitObject(Message) OtherActor)
  (Actor|DestroyActor))

(event EventBeginPlay
  (Utilities|FlowControl|Delay (Variables|Default|GetExplodeTime))
  (Effects|SpawnEmitteratLocation "/Game/StarterContent/Particles/P_Explosion.P_Explosion" (Transformation|GetWorldLocation (Variables|Default|GetStaticMesh)))
  (Actor|DestroyActor))

(event EventActorBeginOverlap
  (params (OtherActor :type Actor%20Object%20Reference))
  (Effects|SpawnEmitteratLocation "/Game/StarterContent/Particles/P_Explosion.P_Explosion" (Transformation|GetWorldLocation (Variables|Default|GetStaticMesh)))
  (Class|BPIExplodable|ProjectileHitObject(Message) (stale OnComponentHit(StaticMesh) OtherActor))
  (Actor|DestroyActor))

(event EventTick
  (params (DeltaSeconds :type Float%20%28single-precision%29))
  (Physics|SetPhysicsLinearVelocity (Variables|Default|GetStaticMesh) (Math|Vector|RotateVector (Math|Vector|MakeVector (Variables|Default|GetAcceleration) 0.0 0.0) (Transformation|GetActorRotation)) true "None"))

(fn ConstructionScript)

(fn Explode
  (Effects|SpawnEmitteratLocation "/Game/StarterContent/Particles/P_Explosion.P_Explosion" (Transformation|GetActorLocation)))