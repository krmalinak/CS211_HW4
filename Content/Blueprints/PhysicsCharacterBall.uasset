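; A physics-driven ball character that rolls by applying torque to its mesh.
; Each tick, forward and right movement inputs form a torque vector, rotated by the camera's world rotation so rolling is view-relative.
; The TurnRate axis yaws the spring arm, scaled by delta time and a turn-rate scalar.
; BeginPlay sets the player camera manager to follow HMD orientation for VR.
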(event EventBeginPlay
  (Variables|/Script/Engine.PlayerCameraManager|SetbFollowHmdOrientation (Game|GetPlayerCameraManager 0) true))

(event EventTick
  (params (DeltaSeconds :type Float%20%28single-precision%29))
  (Class|PrimitiveComponent|AddTorque (Variables|Default|GetBallMesh) (Math|Vector|RotateVector (Math|Vector|MakeVector (* (Variables|Default|GetTorque) (Input|AxisValues|GetMoveRight) -1.0) (* (Variables|Default|GetTorque) (Input|AxisValues|GetMoveForward) 1.0) 0.0) (Transformation|GetWorldRotation (Variables|Default|GetCamera))) "None"))

(event Input|AxisEvents|InputAxisTurnRate
  (params (AxisValue :type Float%20%28single-precision%29))
  (Transformation|AddWorldRotation (Variables|Default|GetSpringArm) (Math|Rotator|MakeRotator 0.0 (* AxisValue (Utilities|Time|GetWorldDeltaSeconds) (Variables|Default|GetTurnRateScalar)) 0.0) false))

(fn ConstructionScript)